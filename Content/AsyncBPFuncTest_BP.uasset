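; Test actor for running Blueprint logic off the game thread, logging thread IDs and showing progress in a widget.
; Key 1 runs TestFunc by name as a heavy async loop.
; Key 2 runs an event on a new thread with game-thread and finish callbacks.
; Key 4 loops a prime calculator on a runnable thread, sending results to the widget until a critical event ends it at a count limit.
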(event Custom|EventOnNewThread
  (params (objs :type Array%20of%20Object%20Object%20References))
  ;[1 1 1] Start Async Func With Option
  (bind _returnvalue (Class|AsyncBpLibrary|GetNowThreadId))
  (Development|PrintString (Utilities|String|Append "new thread 1 :" (Utilities|String|ToString(Integer) _returnvalue)))
  (Class|AsyncBpLibrary|MakeCurrentThreadSleep 1.0)
  (Class|AsyncFuncWorker|ExecuteGameThreadEventonGameThread (Variables|Default|GetAsyncFuncWorker))
  (Class|AsyncBpLibrary|MakeCurrentThreadSleep 2.0)
  (bind _returnvalue_2 (Class|AsyncBpLibrary|GetNowThreadId))
  (Development|PrintString (Utilities|String|Append "new thread 2:" (Utilities|String|ToString(Integer) _returnvalue_2))))

(event Custom|EventOnGameThread
  (params (objs :type Array%20of%20Object%20Object%20References))
  ;[1 1 1] Start Async Func With Option
  (bind _returnvalue (Class|AsyncBpLibrary|GetNowThreadId))
  (Development|PrintString (Utilities|String|Append "call back to game thread111 :" (Utilities|String|ToString(Integer) _returnvalue)))
  (Class|AsyncBpLibrary|MakeCurrentThreadSleep 2.0)
  (bind _returnvalue_2 (Class|AsyncBpLibrary|GetNowThreadId))
  (Development|PrintString (Utilities|String|Append "call back to game thread2222 :" (Utilities|String|ToString(Integer) _returnvalue_2))))

(event Custom|GameThreadEVt1
  (params (intArray :type Array%20of%20Integers) (floatArray :type Array%20of%20Floats%20%28single-precision%29) (StringArray :type Array%20of%20Strings))
  (bind _output (Utilities|Array|Get(acopy) intArray 1))
  (bind _output_2 (Utilities|Array|Get(acopy) intArray))
  (bind _returnvalue (Utilities|String|ToString(Integer) _output_2))
  (bind _returnvalue_2 (Utilities|String|ToString(Integer) _output))
  (bind _returnvalue_3 (Utilities|String|Append "mission id:" _returnvalue "    now num:" _returnvalue_2))
  (Math|Integer|IncrementInt (Variables|Default|GetTestRunnable_MissonCounter)
    (:%20%20
      (if (> (Utilities|Array|Length intArray) 1)
        (Development|PrintString (Utilities|String|Append "game thread evt:" _returnvalue_3))
        (Rendering|Components|TextRender|SetText (Variables|/AsyncFuncCaller/TestThread_Wdb.TestThread_Wdb_C|GetTextBlock_90 (Variables|Default|GetTestThreadWdb)) (Utilities|Text|ToText(String) _returnvalue_3))))))

(event Custom|OnFinish
  (params (objs :type Array%20of%20Object%20Object%20References))
  ;[1 1 1] Start Async Func With Option
  (bind _returnvalue (Class|AsyncBpLibrary|GetNowThreadId))
  (Development|PrintString (Utilities|String|Append "on finish :" (Utilities|String|ToString(Integer) _returnvalue))))

(event Custom|CriticalEvt
  (params (objs :type Array%20of%20Object%20Object%20References))
  (bind _asprime_num_calculator (Utilities|Casting|CastToPrimeNumCalculator (Utilities|Array|Get(acopy) objs)))
  (Development|PrintString (Utilities|String|Append "critical event  counter :" (Utilities|String|ToString(Integer) (Variables|/AsyncFuncCaller/PrimeNumCalculator.PrimeNumCalculator_C|GetMissonCounter _asprime_num_calculator))))
  (if (>= (Variables|/AsyncFuncCaller/PrimeNumCalculator.PrimeNumCalculator_C|GetMissonCounter _asprime_num_calculator) 499)
    (Development|PrintString "loop end thread")
    (Class|RunnableThreadCaller|EndThread (Variables|Default|GetRunnableThreadWorker))))

(event Custom|AsyncEvt
  (params (objs :type Array%20of%20Object%20Object%20References))
  (bind _runnablethreadworker (Variables|Default|GetRunnableThreadWorker))
  (bind _asprime_num_calculator (Utilities|Casting|CastToPrimeNumCalculator (Utilities|Array|Get(acopy) objs)))
  (Class|RunnableThreadCaller|ExecuteCriticalEvent _runnablethreadworker)
  (Default|CaculateNextPrimNumber _asprime_num_calculator)
  (Development|PrintString "Hello")
  (Class|RunnableThreadCaller|ExecuteGameThreadEvent _runnablethreadworker (Utilities|Array|MakeArray (Variables|/AsyncFuncCaller/PrimeNumCalculator.PrimeNumCalculator_C|GetMissonCounter _asprime_num_calculator) (Variables|/AsyncFuncCaller/PrimeNumCalculator.PrimeNumCalculator_C|GetNowPrimeNumber _asprime_num_calculator)) (Utilities|Array|MakeArray) (Utilities|Array|MakeArray)))

(event Custom|FinishEvent
  (params (objs :type Array%20of%20Object%20Object%20References))
  (bind _asprime_num_calculator (Utilities|Casting|CastToPrimeNumCalculator (Utilities|Array|Get(acopy) objs)))
  (Rendering|Components|TextRender|SetText (Variables|/AsyncFuncCaller/TestThread_Wdb.TestThread_Wdb_C|GetTextBlock_90 (Variables|Default|GetTestThreadWdb)) (Utilities|Text|ToText(String) (Utilities|String|Append "mission id:" (Utilities|String|ToString(Integer) (Variables|/AsyncFuncCaller/PrimeNumCalculator.PrimeNumCalculator_C|GetMissonCounter _asprime_num_calculator)) "    now num:" (Utilities|String|ToString(Integer) (Variables|/AsyncFuncCaller/PrimeNumCalculator.PrimeNumCalculator_C|GetNowPrimeNumber _asprime_num_calculator)) "   over!!!"))))

(event EventBeginPlay
  ;[1 1 1] Begin Play
  (Input|EnableInput (Game|GetPlayerController 0))
  (bind _returnvalue (UserInterface|CreateWidget "/AsyncFuncCaller/TestThread_Wdb.TestThread_Wdb_C" (Game|GetPlayerController 0)))
  (UserInterface|Viewport|AddtoViewport _returnvalue 0)
  (Variables|Default|SetTestThreadWdb _returnvalue))

(event EventEndPlay
  (params (EndPlayReason :type EEndPlayReason%20Enum :default "Destroyed"))
  (bind _runnablethreadworker (Variables|Default|GetRunnableThreadWorker))
  ;[1 1 1] End Play Event
  (Utilities|FlowControl|Sequence
    (:then_0
      (Utilities|IsValid _runnablethreadworker
        (:Is%20Valid
          (Class|RunnableThreadCaller|EndThread _runnablethreadworker))))
    (:then_1
      (Class|AsyncBpLibrary|ReleaseUObject (Variables|Default|GetLoopEventManager)))))

(event Input|KeyboardEvents|1
  (params (Key :type Key%20Structure :default "None"))
  ;[1 1 1] Start Async func by func name
  (:Pressed
    (bind _returnvalue (Class|AsyncBpLibrary|GetNowThreadId))
    (Development|PrintString (Utilities|String|Append "Start Test Func 1, main game thread:" (Utilities|String|ToString(Integer) _returnvalue)))
    (bind _obj (|StartAsyncFuncbyFuncName "TestFunc" self)
      (:then
        (Development|PrintString "call over"))
      (:OnComplete
        (bind _asasync_bpfunc_test_bp (Utilities|Casting|CastToAsyncBPFuncTest_BP _obj))
        (bind _returnvalue_2 (Class|AsyncBpLibrary|GetNowThreadId))
        (Development|PrintString (Utilities|String|Append "complete , obj  is:" (Utilities|String|ToString(Object) _asasync_bpfunc_test_bp) "    ---res:" (Utilities|String|ToString(Float) (Variables|AsyncBPFuncTest_BP_C|GetRes _asasync_bpfunc_test_bp)) "     main thread id :" (Utilities|String|ToString(Integer) _returnvalue_2)))))))

(event Input|KeyboardEvents|2
  (params (Key :type Key%20Structure :default "None"))
  ;[1 1 1] Start Async Func With Option
  (:Pressed
    (bind _returnvalue (Class|AsyncBpLibrary|GetNowThreadId))
    (Development|PrintString (Utilities|String|Append "start async :" (Utilities|String|ToString(Integer) _returnvalue)))
    (bind _returnvalue_2 (Class|AsyncBpLibrary|StartAsyncFuncwithOption (Utilities|Struct|MakeAsyncFuncOption (Utilities|Array|MakeArray) (delegate Custom|EventOnNewThread) (delegate Custom|EventOnGameThread) (delegate Custom|OnFinish))))
    (Variables|Default|SetAsyncFuncWorker _returnvalue_2)))

(event Input|KeyboardEvents|3
  (params (Key :type Key%20Structure :default "None"))
  ;[1 1 1] Start RunnableThread With Option
)

(event Input|KeyboardEvents|4
  (params (Key :type Key%20Structure :default "None"))
  (:Pressed
    (bind _returnvalue (Class|AsyncLoopEventManager|CreateAAsyncLoopEventManager))
    (bind _output_get (Variables|Default|SetLoopEventManager _returnvalue))
    (bind _returnvalue_2 (Game|ConstructObjectfromClass "/AsyncFuncCaller/PrimeNumCalculator.PrimeNumCalculator_C" self))
    (bind _returnvalue_3 (Class|AsyncLoopEventManager|StartAsyncLoopEvent _output_get (Utilities|Struct|MakeRunnableThreadOption (Utilities|Array|MakeArray _returnvalue_2) (delegate Custom|CriticalEvt) (delegate Custom|AsyncEvt) (delegate Custom|GameThreadEVt1) (delegate Custom|FinishEvent))))
    (Variables|Default|SetRunnableThreadWorker _returnvalue_3)))

(fn ConstructionScript)

(fn TestFunc
  (bind _returnvalue (Class|AsyncBpLibrary|GetNowThreadId))
  (Development|PrintString (Utilities|String|Append "async Start Test Func 1, thread id :" (Utilities|String|ToString(Integer) _returnvalue)))
  (for _index (range 0 100000)
    (for _index_2 (range 0 _index)
      (Variables|Default|SetRes (+ (Math|Conversions|ToFloat(Integer) (Math|Conversions|ToInteger(Byte) (Utilities|String|ToString(Float) (Math|Conversions|ToFloat(Integer) _index_2)))) (Variables|Default|GetRes)))))
  (return))